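; BP_WoodenShelf_01 is a wooden shelf prop with two doors whose opening is set by variables.
; The construction script sets each door's yaw from Door01Open or Door02Open, negating the right one and adding a 90-degree offset to both.
; It uses world rotation, so the door angles ignore the actor's own rotation.
; The event graph holds only disabled placeholder events, so there is no runtime logic.
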(fn `UserConstructionScript`
  (`SceneComponent.K2_SetWorldRotation` (`self.WoodenShelf_Door_L`) (`KismetMathLibrary.MakeRotator` 0.0 0.0 (+ (`self.Door_01_Open`) 90.0)) false false)
  (`SceneComponent.K2_SetWorldRotation` (`self.WoodenShelf_Door_R`) (`KismetMathLibrary.MakeRotator` 0.0 0.0 (+ (* (`self.Door_02_Open`) -1.0) 90.0)) false false))